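; Behavior tree task that moves the turtle2 AI pawn along world Y in a two-phase, timed rhythm.
; A flag alternates between a one-second phase at Speed1 and a half-second phase at Speed2, timed with UTC timestamps.
; Each execution adds forced movement input or, when the phase expires, flips it and plays a footstep sound at the pawn.
; The task finishes successfully every time, relying on repeated execution for continuous motion.
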(event EventReceiveExecuteAI
  (params (OwnerController :type AI%20Controller%20Object%20Reference) (ControlledPawn :type Pawn%20Object%20Reference))
  (bind _returnvalue (Transformation|GetActorLocation ControlledPawn))
  (if (Variables|Default|Getflag)
    (if (< (- (Math|DateTime|UTCNow) (Variables|Default|Gettime1)) (Math|Timespan|MakeTimespan 0 0 0 0 1000))
      (Pawn|Input|AddMovementInput ControlledPawn "0,1.000000, 0" (Variables|Default|Getspeed1) true)
      (else
        (Variables|Default|Setflag false)
        (Variables|Default|Settime2 (Math|DateTime|UTCNow))
        (Audio|PlaySoundatLocation "/Game/Assets/sounds/feet-footsteps-wood-parquet.feet-footsteps-wood-parquet" _returnvalue "0, 0, 0" 1.0 1.0 0.0 0 0 0)))
    (AI|BehaviorTree|FinishExecute true)
    (else
      (if (< (- (Math|DateTime|UTCNow) (Variables|Default|Gettime2)) (Math|Timespan|MakeTimespan 0 0 0 0 500))
        (Pawn|Input|AddMovementInput ControlledPawn "0,1.000000, 0" (Variables|Default|Getspeed2) true)
        (else
          (Variables|Default|Setflag true)
          (Variables|Default|Settime1 (Math|DateTime|UTCNow))
          (Audio|PlaySoundatLocation "/Game/Assets/sounds/feet-footsteps-wood-parquet.feet-footsteps-wood-parquet" _returnvalue "0, 0, 0" 1.0 1.0 0.0 0 0 0)))
      (AI|BehaviorTree|FinishExecute true))))